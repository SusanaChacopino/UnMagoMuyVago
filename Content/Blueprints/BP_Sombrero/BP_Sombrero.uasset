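; BP_Sombrero is a VR grabbable hat that disappears once the player's put-on-hat flag (PonerseSombrero) is true.
; On BeginPlay it caches the first VRPawn, then polls that flag with a self-calling event and short delay.
; When the flag is set, it marks SombreroPuesto, prints it and destroys itself.
; GrabComponent events turn the hat mesh's physics off when grabbed and on when dropped.
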(event `self.ReceiveBeginPlay`
  (bind _outactors (`GameplayStatics.GetAllActorsOfClass` "/Game/VRTemplate/Blueprints/VRPawn.VRPawn_C"))
  (bind _output_get (set `self.Ref Jugador` (`|GetArrayItem` _outactors)))
  (`KismetSystemLibrary.PrintString` (`KismetStringLibrary.Conv_ObjectToString` _output_get))
  (`self.PonerseSombrero`))

(event `PonerseSombrero`
  (if (`/Game/VRTemplate/Blueprints/VRPawn.PonerseSombrero` (`self.Ref Jugador`))
    (bind _output_get (set `self.SombreroPuesto` true))
    (`KismetSystemLibrary.PrintString` (`KismetStringLibrary.Conv_BoolToString` _output_get))
    (`self.K2_DestroyActor`)
    (else
      (`KismetSystemLibrary.Delay` 0.2)
      (`self.PonerseSombrero`))))

(event `self.GrabComponent.OnGrabbed`
  (`PrimitiveComponent.SetSimulatePhysics` (`self.Sombrero`) false))

(event `self.GrabComponent.OnDropped`
  (`PrimitiveComponent.SetSimulatePhysics` (`self.Sombrero`) true))

(fn `UserConstructionScript`)