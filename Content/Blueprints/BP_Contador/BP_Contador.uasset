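; BP_Contador is a countdown timer actor that displays remaining time as minutes and zero-padded seconds once the referenced cauldron activates it.
; Tick polls the ActivarContador flag on RefCaldero, and a DoOnce starts the countdown and reveals TextoContador.
; A looping one-second timer decrements TiempoRestante and refreshes the text.
; The countdown has no stop or expiry handling at zero.
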(event `self.ReceiveBeginPlay`)

(event `self.ReceiveTick`
  (params (DeltaSeconds :type "Float (single-precision)"))
  ; Comprobar si se debe iniciar el contador
  (if (`/Game/Blueprints/BP_Caldero/BP_Caldero.ActivarContador` (`self.Ref Caldero`))
    (`/Engine/EditorBlueprintResources/StandardMacros.DoOnce` false
      (:`Completed`
        (`self.IniciarContador`)
        (`SceneComponent.SetVisibility` (`self.TextoContador`) true false)))))

(event `IniciarContador`
  ; Crear y Restar al contador
  (`KismetSystemLibrary.K2_SetTimerDelegate` (delegate `RestarAlContador`) 1.0 true))

(event `RestarAlContador`
  ; Crear y Restar al contador
  (set `self.TiempoRestante` (- (`self.TiempoRestante`) 1))
  (set `self.Minutos` (/ (`self.TiempoRestante`) 60))
  (set `self.Segundos` (mod (`self.TiempoRestante`) 60))
  (if (< (`self.Segundos`) 10)
    (set `self.TextoSegundos` (`|FormatText` "0{Segundos}" (`self.Segundos`)))
    (else
      (set `self.TextoSegundos` (`|GenericToText` (`self.Segundos`)))))
  (`TextRenderComponent.K2_SetText` (`self.TextoContador`) (`|FormatText` "{Minutos}:{TextoSegundos}" (`self.Minutos`) (`self.TextoSegundos`))))

(fn `UserConstructionScript`)