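; VR book actor whose cover opens and closes with animations when its left and right trigger volumes are overlapped in sequence.
; Each side sets a flag, so right-then-left opens a closed cover and left-then-right closes an open one at negative play rate.
; BeginPlay plays the idle animation and caches the VRPawn.
; Page-turn logic for two pages exists but is disconnected, and both overlaps print debug strings.
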(event `self.ReceiveBeginPlay`
  (`SkeletalMeshComponent.PlayAnimation` (`self.Libro`) "/Game/Assets/libro/nuevolibro/libro_entero_Anim_Idle.libro_entero_Anim_Idle" false)
  (bind _asvrpawn (cast `/Game/VRTemplate/Blueprints/VRPawn` (`GameplayStatics.GetPlayerPawn` 0)))
  (set `self.Ref Jugador` _asvrpawn))

(event `self.LadoDerecho.OnComponentBeginOverlap`
  (params (OverlappedComponent :type "PrimitiveComponent Object Reference") (OtherActor :type "Actor Object Reference") (OtherComp :type "PrimitiveComponent Object Reference") (OtherBodyIndex :type Integer) (bFromSweep :type Boolean) (SweepResult :type "HitResult Structure (by ref)"))
  (`KismetSystemLibrary.PrintString` "a")
  (if (`self.LadoIzquierdoOverlap`)
    (if (`self.PortadaAbierta`)
      (`SkeletalMeshComponent.SetPlayRate` (`self.Libro`) -1.0)
      (`SkeletalMeshComponent.PlayAnimation` (`self.Libro`) "/Game/Assets/libro/nuevolibro/libro_entero_Anim_abrirPortadaCerrandose.libro_entero_Anim_abrirPortadaCerrandose" false)
      (set `self.PortadaAbierta` false)
      (set `self.LadoIzquierdoOverlap` false)
      (set `self.LadoDerechoOverlap` false))
    (else
      (set `self.LadoDerechoOverlap` true))))

(event `self.LadoIzquierdo.OnComponentBeginOverlap`
  (params (OverlappedComponent :type "PrimitiveComponent Object Reference") (OtherActor :type "Actor Object Reference") (OtherComp :type "PrimitiveComponent Object Reference") (OtherBodyIndex :type Integer) (bFromSweep :type Boolean) (SweepResult :type "HitResult Structure (by ref)"))
  (`KismetSystemLibrary.PrintString` "b")
  (if (`self.LadoDerechoOverlap`)
    (if (not (`self.PortadaAbierta`))
      (`SkeletalMeshComponent.SetPlayRate` (`self.Libro`) 1.0)
      (`SkeletalMeshComponent.PlayAnimation` (`self.Libro`) "/Game/Assets/libro/nuevolibro/libro_entero_Anim_abrirPortada.libro_entero_Anim_abrirPortada" false)
      (set `self.PortadaAbierta` true)
      (set `self.LadoIzquierdoOverlap` false)
      (set `self.LadoDerechoOverlap` false))
    (else
      (set `self.LadoIzquierdoOverlap` true))))

(fn `UserConstructionScript`)