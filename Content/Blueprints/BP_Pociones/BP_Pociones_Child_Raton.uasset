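; Mouse potion for VR, a child potion Blueprint that turns the player's VRPawn into a mouse.
; Grabbing it enables input, so the right index-curl action calls ConvertirseEnRaton on the cached pawn.
; That press also feeds a DoOnce that runs the pawn's EfectoRaton effect for three seconds.
; Dropping it disables input and resets the DoOnce, limiting the effect to once per grab.
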(event `self.ReceiveBeginPlay`
  (bind _asvrpawn (cast `/Game/VRTemplate/Blueprints/VRPawn` (`GameplayStatics.GetPlayerPawn` 0)))
  (set `self.Ref VRPawn` _asvrpawn))

(event `self.GrabComponent.OnGrabbed`
  (`self.EnableInput` (`GameplayStatics.GetPlayerController` 0))
  (set `self.CogiendoPocion` true))

(event `self.GrabComponent.OnDropped`
  (`self.DisableInput` (`GameplayStatics.GetPlayerController` 0))
  (set `self.CogiendoPocion` false)
  (goto _label :!via `Reset`))

(event `EnhancedInput|/Game/VRTemplate/Input/Actions/Hands/IA_Hand_IndexCurl_Left`
  (params (ActionValue :type "Float (double-precision)") (ElapsedSeconds :type "Float (double-precision)") (TriggeredSeconds :type "Float (double-precision)") (InputAction :type "InputAction Object Reference" :default "/Game/VRTemplate/Input/Actions/Hands/IA_Hand_IndexCurl_Left.IA_Hand_IndexCurl_Left")))

(event `EnhancedInput|/Game/VRTemplate/Input/Actions/Hands/IA_Hand_IndexCurl_Right`
  (params (ActionValue :type "Float (double-precision)") (ElapsedSeconds :type "Float (double-precision)") (TriggeredSeconds :type "Float (double-precision)") (InputAction :type "InputAction Object Reference" :default "/Game/VRTemplate/Input/Actions/Hands/IA_Hand_IndexCurl_Right.IA_Hand_IndexCurl_Right"))
  (:`Triggered`
    (`/Game/VRTemplate/Blueprints/VRPawn.ConvertirseEnRaton` (`self.Ref VRPawn`))
    (`/Engine/EditorBlueprintResources/StandardMacros.DoOnce` false :!label _label
      (:`Completed`
        (`ActorComponent.Activate` (`/Game/VRTemplate/Blueprints/VRPawn.EfectoRaton` (`self.Ref VRPawn`)) false)
        (`KismetSystemLibrary.Delay` 3.0)
        (`ActorComponent.Deactivate` (`/Game/VRTemplate/Blueprints/VRPawn.EfectoRaton` (`self.Ref VRPawn`)))))))

(fn `UserConstructionScript`
  (`parent.UserConstructionScript`))