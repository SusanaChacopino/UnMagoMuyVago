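; VR gravity wand that pulls and holds physics objects remotely while the player carries it.
; Grabbing or dropping the wand via GrabComponentSnap toggles its input.
; Either index trigger line-traces forward from PosicionObjeto, with longer reach on the left, grabs simulating components through a PhysicsHandle and activates the Rayo beam; release undoes both.
; Tick drives the handle target and active beam's end to PosicionObjeto.
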(event `EnhancedInput|/Game/VRTemplate/Input/Actions/Hands/IA_Hand_IndexCurl_Left`
  (params (ActionValue :type "Float (double-precision)") (ElapsedSeconds :type "Float (double-precision)") (TriggeredSeconds :type "Float (double-precision)") (InputAction :type "InputAction Object Reference" :default "/Game/VRTemplate/Input/Actions/Hands/IA_Hand_IndexCurl_Left.IA_Hand_IndexCurl_Left"))
  (bind _posicionobjeto (`self.PosicionObjeto`))
  (bind _returnvalue (`SceneComponent.K2_GetComponentLocation` _posicionobjeto))
  (:`Triggered`
    (`KismetSystemLibrary.PrintString` "pulsando gatillo")
    (bind (_outhit _returnvalue_2) (`KismetSystemLibrary.LineTraceSingle` _returnvalue (+ _returnvalue (* (`SceneComponent.GetForwardVector` _posicionobjeto) (`KismetMathLibrary.Conv_DoubleToVector` 1000.0))) "TraceTypeQuery1"))
    (if _returnvalue_2
      (bind (_bblockinghit _binitialoverlap _time _distance _location _impactpoint _normal _impactnormal _physmat _hitactor _hitcomponent) (`GameplayStatics.BreakHitResult` _outhit))
      (if (`SceneComponent.IsSimulatingPhysics` _hitcomponent "None")
        (`PhysicsHandleComponent.GrabComponentAtLocation` (`self.PhysicsHandle`) _hitcomponent "None" (`SceneComponent.K2_GetComponentLocation` _hitcomponent))
        (`KismetSystemLibrary.PrintString` "cogiendo objeto")
        (`ActorComponent.Activate` (`self.Rayo`) false)
        (else
          (`KismetSystemLibrary.PrintString` "el actor no es valido")))))
  (:`Completed`
    (`PhysicsHandleComponent.ReleaseComponent` (`self.PhysicsHandle`))
    (`ActorComponent.Deactivate` (`self.Rayo`))))

(event `EnhancedInput|/Game/VRTemplate/Input/Actions/Hands/IA_Hand_IndexCurl_Right`
  (params (ActionValue :type "Float (double-precision)") (ElapsedSeconds :type "Float (double-precision)") (TriggeredSeconds :type "Float (double-precision)") (InputAction :type "InputAction Object Reference" :default "/Game/VRTemplate/Input/Actions/Hands/IA_Hand_IndexCurl_Right.IA_Hand_IndexCurl_Right"))
  (bind _posicionobjeto (`self.PosicionObjeto`))
  (bind _returnvalue (`SceneComponent.K2_GetComponentLocation` _posicionobjeto))
  (:`Triggered`
    (`KismetSystemLibrary.PrintString` "pulsando gatillo")
    (bind (_outhit _returnvalue_2) (`KismetSystemLibrary.LineTraceSingle` _returnvalue (+ _returnvalue (* (`SceneComponent.GetForwardVector` _posicionobjeto) (`KismetMathLibrary.Conv_DoubleToVector` 500.0))) "TraceTypeQuery1"))
    (if _returnvalue_2
      (bind (_bblockinghit _binitialoverlap _time _distance _location _impactpoint _normal _impactnormal _physmat _hitactor _hitcomponent) (`GameplayStatics.BreakHitResult` _outhit))
      (if (`SceneComponent.IsSimulatingPhysics` _hitcomponent "None")
        (`PhysicsHandleComponent.GrabComponentAtLocation` (`self.PhysicsHandle`) _hitcomponent "None" (`SceneComponent.K2_GetComponentLocation` _hitcomponent))
        (`KismetSystemLibrary.PrintString` "cogiendo objeto")
        (`ActorComponent.Activate` (`self.Rayo`) false)
        (else
          (`KismetSystemLibrary.PrintString` "el actor no es valido")))))
  (:`Completed`
    (`PhysicsHandleComponent.ReleaseComponent` (`self.PhysicsHandle`))
    (`ActorComponent.Deactivate` (`self.Rayo`))))

(event `self.ReceiveTick`
  (params (DeltaSeconds :type "Float (single-precision)"))
  (`PhysicsHandleComponent.SetTargetLocation` (`self.PhysicsHandle`) (`SceneComponent.K2_GetComponentLocation` (`self.PosicionObjeto`)))
  (if (`ActorComponent.IsActive` (`self.Rayo`))
    (`NiagaraComponent.SetVariablePosition` (`self.Rayo`) "Beam END" (`SceneComponent.K2_GetComponentLocation` (`self.PosicionObjeto`)))))

(event `self.GrabComponentSnap.OnGrabbed`
  (`self.EnableInput` (`GameplayStatics.GetPlayerController` 0)))

(event `self.GrabComponentSnap.OnDropped`
  (`self.DisableInput` (`GameplayStatics.GetPlayerController` 0)))

(fn `UserConstructionScript`)