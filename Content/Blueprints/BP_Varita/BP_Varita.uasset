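; BP_Varita is a wand that, when grabbed, tries to pick up the ingredient it points at.
; GrabComponent events toggle mesh physics, and grabbing starts IntentarAgarrarObjeto, a delay-driven loop that keeps retrying and has no stop on drop.
; It traces from PuntaVarita and hands hits matching ClaseBPIngrediente to a PhysicsHandle, which is never released here.
; The trace's start and end are the same forward-offset point, giving it zero length.
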(event `self.ReceiveBeginPlay`
  (`self.EnableInput` (`GameplayStatics.GetPlayerController` 0)))

(event `self.GrabComponent.OnDropped`
  (`PrimitiveComponent.SetSimulatePhysics` (`self.StaticMesh`) true))

(event `self.GrabComponent.OnGrabbed`
  (`PrimitiveComponent.SetSimulatePhysics` (`self.StaticMesh`) false)
  (`self.IntentarAgarrarObjeto`))

(event `IntentarAgarrarObjeto`
  (bind _puntavarita (`self.PuntaVarita`))
  (bind _returnvalue (+ (`SceneComponent.K2_GetComponentLocation` _puntavarita) (* (`SceneComponent.GetForwardVector` _puntavarita) 2000)))
  (bind (_outhit _returnvalue_2) (`KismetSystemLibrary.LineTraceSingle` :`Start` _returnvalue :`End` _returnvalue :`TraceChannel` "TraceTypeQuery1" :`DrawDebugType` "ForDuration"))
  (if _returnvalue_2
    (bind (_bblockinghit _binitialoverlap _time _distance _location _impactpoint _normal _impactnormal _physmat _hitactor _hitcomponent) (`GameplayStatics.BreakHitResult` _outhit))
    (if (== _hitactor (`self.Clase BP_Ingrediente`))
      (`KismetSystemLibrary.PrintString` "Apuntando")
      (`PhysicsHandleComponent.GrabComponentAtLocation` (`self.PhysicsHandle`) _hitcomponent "None" _impactpoint)
      (`KismetSystemLibrary.Delay` 3.0)
      (`self.IntentarAgarrarObjeto`)
      (else
        (`KismetSystemLibrary.Delay` 0.2)
        (`self.IntentarAgarrarObjeto`)
        (`KismetSystemLibrary.PrintString` "No se a apuntado")))
    (else
      (`KismetSystemLibrary.PrintString` "no ha habido colision")
      (`KismetSystemLibrary.Delay` 2.0)
      (`self.IntentarAgarrarObjeto`))))

(fn `UserConstructionScript`)