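; VR potion-game cauldron that destroys overlapping ingredients and brews love, invisibility, mouse or bad potions, with matching bubble effects.
; Delay-driven recursive events poll per-potion arrays, using destroyed (invalid) references to count progress or rule out recipes.
; Completed recipes launch a physics potion; love and mouse progress also removes crystal-ball hints.
; The first ingredient starts countdown monitoring; timeout can spawn the bad potion, while the Final event is unfinished.
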(event `self.ReceiveBeginPlay`
  (`self.ComprobarPocionEnamoramiento`)
  (`self.ComprobarPocionInvisibilidad`)
  (`self.ComprobarPocionRaton`)
  (`self.ComprobarPocionMala`)
  (`self.CambiarColorBurbujas`)
  (bind _asvrpawn (cast `/Game/VRTemplate/Blueprints/VRPawn` (`GameplayStatics.GetPlayerPawn` 0)))
  (set `self.Ref VRPawn` _asvrpawn))

(event `CambiarColorBurbujas`
  ; Cambiar Color Burbujas Dependiendo De La Pocion Haciendose
  (if (`self.HaciendoPocionAmor?`)
    (`NiagaraComponent.SetAsset` (`self.EfectoBurbujeo`) "/Game/Niaggara/NS_BurbujasCaldero_PocionAmor.NS_BurbujasCaldero_PocionAmor" true)
    (`KismetSystemLibrary.Delay` 1.0)
    (`self.CambiarColorBurbujas`)
    (elif (`self.HaciendoPocionInvisibilidad?`)
      (`NiagaraComponent.SetAsset` (`self.EfectoBurbujeo`) "/Game/Niaggara/NS_BurbujasCaldero_PocionInvisibilidad.NS_BurbujasCaldero_PocionInvisibilidad" true)
      (`KismetSystemLibrary.Delay` 1.0)
      (`self.CambiarColorBurbujas`)
      (elif (`self.HaciendoPocionRaton?`)
        (`NiagaraComponent.SetAsset` (`self.EfectoBurbujeo`) "/Game/Niaggara/NS_BurbujasCaldero_PocionRaton.NS_BurbujasCaldero_PocionRaton" true)
        (`KismetSystemLibrary.Delay` 1.0)
        (`self.CambiarColorBurbujas`)
        (elif (`self.HaciendoPocionMala`)
          (`NiagaraComponent.SetAsset` (`self.EfectoBurbujeo`) "/Game/Niaggara/NS_BurbujasCaldero_PocionMala.NS_BurbujasCaldero_PocionMala" true)
          (`KismetSystemLibrary.Delay` 1.0)
          (`self.CambiarColorBurbujas`)
          (else
            (`NiagaraComponent.SetAsset` (`self.EfectoBurbujeo`) "/Game/Niaggara/NS_BurbujasCalderoNormal.NS_BurbujasCalderoNormal" true)
            (`KismetSystemLibrary.Delay` 1.0)
            (`self.CambiarColorBurbujas`)))))))

(event `ComprobarPocionEnamoramiento`
  (bind _ingredientespocionenamoramiento (`self.IngredientesPocionEnamoramiento`))
  (bind _particulaspocionterminada (`self.ParticulasPocionTerminada`))
  (bind _particulaspocionterminada_2 (`self.ParticulasPocionTerminada`))
  (bind _arraypistasamor (`/Game/Blueprints/BP_BolaCristal/BP_BolaCristal.ArrayPistasAmor` (`self.Ref BolaCristal`)))
  ; Comprobar Si el Nuevo Ingrediente Es Parte De La Pocion De Enamoramiento
  (`KismetSystemLibrary.PrintString` "Comprobando Ingrediente")
  (if (== (`self.IngredientesRestantesPocionEnamoramiento`) 0)
    (`KismetSystemLibrary.PrintString` "Spawneando ingrediente")
    (`ParticleSystemComponent.SetTemplate` _particulaspocionterminada "/Game/FXVarietyPack/Particles/P_ky_darkStorm.P_ky_darkStorm")
    (`ActorComponent.Activate` _particulaspocionterminada false)
    (`ParticleSystemComponent.SetTemplate` _particulaspocionterminada_2 "/Game/FXVarietyPack/Particles/P_ky_fireStorm.P_ky_fireStorm")
    (`ActorComponent.Activate` _particulaspocionterminada_2 false)
    (bind _returnvalue (`|SpawnActorFromClass` "/Game/Blueprints/BP_Pociones/BP_Pociones_Child_Enamoramiento.BP_Pociones_Child_Enamoramiento_C" (`KismetMathLibrary.Conv_VectorToTransform` (`self.K2_GetActorLocation` (`self.PosicionSpawnPocion`))) "Undefined" "MultiplyWithRoot" null null))
    (bind _output_get (set `self.RefPocionEnamoramiento` _returnvalue))
    (bind _staticmesh (`/Game/Blueprints/BP_Pociones/BP_Pociones.StaticMesh` _output_get))
    (`PrimitiveComponent.SetSimulatePhysics` _staticmesh true)
    (`PrimitiveComponent.AddImpulse` _staticmesh (500.0 500.0 500.0) "None" false)
    (set `self.PocionAmorTerminada` true)
    (`KismetSystemLibrary.Delay` 2.0)
    (`ActorComponent.Deactivate` (`self.ParticulasPocionTerminada`))
    (`GameplayStatics.PlaySound2D` "/Game/Audios/AudiosBolaCristal/CrearPocionAmor.CrearPocionAmor" 1.0 1.0 0.0 null null)
    (else
      (`KismetSystemLibrary.PrintString` "Comprobando si hay un nuevo ingrediente en caldero")
      (if (`self.NuevoIngredienteEnCaldero`)
        (for _array_element (`self.NOIngredientesPocionEnamoramiento`)
          (`/Engine/EditorBlueprintResources/StandardMacros.IsValid` _array_element
            (:`Is Not Valid`
              (set `self.NOSePuedeHacerPocionEnamoramiento` true)
              (`KismetSystemLibrary.PrintString` "Ingrediente no parte de pocion de enamoramiento"))))
        (if (`self.NOSePuedeHacerPocionEnamoramiento`)
          (`KismetSystemLibrary.PrintString` "No se puede hacer pocion enamoramiento")
          (set `self.HaciendoPocionAmor?` false)
          (else
            (for (_array_element_2 _array_index) _ingredientespocionenamoramiento
              (`/Engine/EditorBlueprintResources/StandardMacros.IsValid` _array_element_2
                (:`Is Valid`
                  (`KismetSystemLibrary.Delay` 1.0)
                  (`self.ComprobarPocionEnamoramiento`)
                  (`KismetSystemLibrary.PrintString` "IngredientenNoDestruido"))
                (:`Is Not Valid`
                  (`KismetArrayLibrary.Array_RemoveItem` _ingredientespocionenamoramiento _array_element_2)
                  (bind _result (`/Engine/EditorBlueprintResources/StandardMacros.DecrementInt` (`self.IngredientesRestantesPocionEnamoramiento`))
                    (:`  `
                      (`KismetSystemLibrary.PrintString` (`KismetStringLibrary.Conv_IntToString` _result))
                      (set `self.HaciendoPocionAmor?` true)
                      (set `self.NuevoIngredienteEnCaldero` false)
                      (`KismetSystemLibrary.Delay` 1.0)
                      (`self.ComprobarPocionEnamoramiento`)
                      (`KismetArrayLibrary.Array_RemoveItem` _arraypistasamor (`|GetArrayItem` _arraypistasamor _array_index))
                      (if (not (`/Game/Blueprints/BP_BolaCristal/BP_BolaCristal.AudioHasFalladoYaDicho` (`self.Ref BolaCristal`)))
                        (`/Engine/EditorBlueprintResources/StandardMacros.DoOnce` false
                          (:`Completed`
                            (`GameplayStatics.PlaySound2D` "/Game/Audios/AudiosBolaCristal/EmpezarHacerPocionAmor.EmpezarHacerPocionAmor" 1.0 1.0 0.0 null null)))))))))))
        (else
          (`KismetSystemLibrary.Delay` 1.0)
          (`self.ComprobarPocionEnamoramiento`))))))

(event `ComprobarPocionInvisibilidad`
  (bind _ingredientespocioninvisibilidad (`self.IngredientesPocionInvisibilidad`))
  (bind _particulaspocionterminada (`self.ParticulasPocionTerminada`))
  ; Comprobar Si el Nuevo Ingrediente Es Parte De La Pocion De Invisibilidad
  (`KismetSystemLibrary.PrintString` "Comprobando Ingrediente")
  (if (<= (`self.IngredientesRestantesPocionInvisibilidad`) 0)
    (`KismetSystemLibrary.PrintString` "Spawneando ingrediente")
    (`ParticleSystemComponent.SetTemplate` _particulaspocionterminada "/Game/FXVarietyPack/Particles/P_ky_aquaStorm.P_ky_aquaStorm")
    (`ActorComponent.Activate` _particulaspocionterminada false)
    (bind _returnvalue (`|SpawnActorFromClass` "/Game/Blueprints/BP_Pociones/BP_Pociones_Child_Invisibilidad.BP_Pociones_Child_Invisibilidad_C" (`KismetMathLibrary.Conv_VectorToTransform` (`self.K2_GetActorLocation` (`self.PosicionSpawnPocion`))) "Undefined" "MultiplyWithRoot" null null))
    (bind _output_get (set `self.RefPocionInvisibilidad` _returnvalue))
    (bind _staticmesh (`/Game/Blueprints/BP_Pociones/BP_Pociones.StaticMesh` _output_get))
    (`PrimitiveComponent.SetSimulatePhysics` _staticmesh true)
    (`PrimitiveComponent.AddImpulse` _staticmesh (500.0 500.0 500.0) "None" false)
    (set `self.PocionInvisibilidadTerminada` true)
    (`KismetSystemLibrary.Delay` 2.0)
    (`ActorComponent.Deactivate` (`self.ParticulasPocionTerminada`))
    (`GameplayStatics.PlaySound2D` "/Game/Audios/AudiosBolaCristal/CrearPocionInvisibilidad.CrearPocionInvisibilidad" 1.0 1.0 0.0 null null)
    (else
      (`KismetSystemLibrary.PrintString` "Comprobando si hay un nuevo ingrediente en caldero")
      (if (`self.NuevoIngredienteEnCaldero`)
        (for _array_element (`self.NOIngredientesPocionInvisibilidad`)
          (`/Engine/EditorBlueprintResources/StandardMacros.IsValid` _array_element
            (:`Is Not Valid`
              (set `self.NOSePuedeHacerPocionInvisibilidad` true)
              (`KismetSystemLibrary.PrintString` "Ingrediente no parte de pocion de enamoramiento"))))
        (if (`self.NOSePuedeHacerPocionInvisibilidad`)
          (`KismetSystemLibrary.PrintString` "No se puede hacer pocion enamoramiento")
          (set `self.HaciendoPocionInvisibilidad?` false)
          (else
            (for _array_element_2 _ingredientespocioninvisibilidad
              (`/Engine/EditorBlueprintResources/StandardMacros.IsValid` _array_element_2
                (:`Is Valid`
                  (`KismetSystemLibrary.Delay` 1.0)
                  (`self.ComprobarPocionInvisibilidad`)
                  (`KismetSystemLibrary.PrintString` "IngredientenNoDestruido"))
                (:`Is Not Valid`
                  (`KismetArrayLibrary.Array_RemoveItem` _ingredientespocioninvisibilidad _array_element_2)
                  (bind _result (`/Engine/EditorBlueprintResources/StandardMacros.DecrementInt` (`self.IngredientesRestantesPocionInvisibilidad`))
                    (:`  `
                      (`KismetSystemLibrary.PrintString` (`KismetStringLibrary.Conv_IntToString` _result))
                      (set `self.HaciendoPocionInvisibilidad?` true)
                      (set `self.NuevoIngredienteEnCaldero` false)
                      (`KismetSystemLibrary.Delay` 1.0)
                      (`self.ComprobarPocionInvisibilidad`)
                      (if (not (`self.PocionRatonTerminada`))
                        (`GameplayStatics.PlaySound2D` "/Game/Audios/AudiosBolaCristal/LoHasHechoMal.LoHasHechoMal" 1.0 1.0 0.0 null null)
                        (set `/Game/Blueprints/BP_BolaCristal/BP_BolaCristal.AudioHasFalladoYaDicho` true (`self.Ref BolaCristal`))))))))))
        (else
          (`KismetSystemLibrary.Delay` 1.0)
          (`self.ComprobarPocionInvisibilidad`))))))

(event `ComprobarPocionRaton`
  (bind _particulaspocionterminada (`self.ParticulasPocionTerminada`))
  (bind _ingredientespocionraton (`self.IngredientesPocionRaton`))
  (bind _arraypistasraton (`/Game/Blueprints/BP_BolaCristal/BP_BolaCristal.ArrayPistasRaton` (`self.Ref BolaCristal`)))
  ; Comprobar Si el Nuevo Ingrediente Es Parte De La Pocion De Raton
  (`KismetSystemLibrary.PrintString` "Comprobando Ingrediente")
  (if (<= (`self.IngredientesRestantesPocionRaton`) 0)
    (`KismetSystemLibrary.PrintString` "Spawneando ingrediente")
    (`ParticleSystemComponent.SetTemplate` _particulaspocionterminada "/Game/FXVarietyPack/Particles/P_ky_thunderStorm.P_ky_thunderStorm")
    (`ActorComponent.Activate` _particulaspocionterminada false)
    (bind _returnvalue (`|SpawnActorFromClass` "/Game/Blueprints/BP_Pociones/BP_Pociones_Child_Raton.BP_Pociones_Child_Raton_C" (`KismetMathLibrary.Conv_VectorToTransform` (`self.K2_GetActorLocation` (`self.PosicionSpawnPocion`))) "Undefined" "MultiplyWithRoot" null null))
    (bind _output_get (set `self.RefPocionRaton` _returnvalue))
    (bind _staticmesh (`/Game/Blueprints/BP_Pociones/BP_Pociones.StaticMesh` _output_get))
    (`PrimitiveComponent.SetSimulatePhysics` _staticmesh true)
    (`PrimitiveComponent.AddImpulse` _staticmesh (500.0 500.0 500.0) "None" false)
    (set `self.PocionRatonTerminada` false)
    (`KismetSystemLibrary.Delay` 2.0)
    (`ActorComponent.Deactivate` (`self.ParticulasPocionTerminada`))
    (`GameplayStatics.PlaySound2D` "/Game/Audios/AudiosBolaCristal/CrearPocionRaton.CrearPocionRaton" 1.0 1.0 0.0 null null)
    (else
      (`KismetSystemLibrary.PrintString` "Comprobando si hay un nuevo ingrediente en caldero")
      (if (`self.NuevoIngredienteEnCaldero`)
        (for _array_element (`self.NOIngredientesPocionRaton`)
          (`/Engine/EditorBlueprintResources/StandardMacros.IsValid` _array_element
            (:`Is Not Valid`
              (set `self.NOSePuedeHacerPocionRaton` true)
              (`KismetSystemLibrary.PrintString` "Ingrediente no parte de pocion de enamoramiento"))))
        (if (`self.NOSePuedeHacerPocionRaton`)
          (`KismetSystemLibrary.PrintString` "No se puede hacer pocion enamoramiento")
          (set `self.HaciendoPocionRaton?` false)
          (else
            (for (_array_element_2 _array_index) _ingredientespocionraton
              (`/Engine/EditorBlueprintResources/StandardMacros.IsValid` _array_element_2
                (:`Is Valid`
                  (`KismetSystemLibrary.Delay` 1.0)
                  (`self.ComprobarPocionRaton`)
                  (`KismetSystemLibrary.PrintString` "IngredientenNoDestruido"))
                (:`Is Not Valid`
                  (`KismetArrayLibrary.Array_RemoveItem` _ingredientespocionraton _array_element_2)
                  (bind _result (`/Engine/EditorBlueprintResources/StandardMacros.DecrementInt` (`self.IngredientesRestantesPocionRaton`))
                    (:`  `
                      (`KismetSystemLibrary.PrintString` (`KismetStringLibrary.Conv_IntToString` _result))
                      (set `self.HaciendoPocionRaton?` true)
                      (set `self.NuevoIngredienteEnCaldero` false)
                      (`KismetSystemLibrary.Delay` 1.0)
                      (`self.ComprobarPocionRaton`)
                      (`KismetArrayLibrary.Array_RemoveItem` _arraypistasraton (`|GetArrayItem` _arraypistasraton _array_index)))))))))
        (else
          (`KismetSystemLibrary.Delay` 1.0)
          (`self.ComprobarPocionRaton`))))))

(event `ComprobarPocionMala`
  (bind _particulaspocionterminada (`self.ParticulasPocionTerminada`))
  ; Comprobar Si Se Tiene Que Spawnear La Pocion Mala Al Acabar El Juego
  (if (and (`self.NOSePuedeHacerPocionRaton`) (`self.NOSePuedeHacerPocionInvisibilidad`) (`self.NOSePuedeHacerPocionEnamoramiento`))
    (set `self.HaciendoPocionMala` true)
    (`self.CambiarColorBurbujas`)
    (if (`self.ElTiempoAAcabado?`) :!label _label
      (`ParticleSystemComponent.SetTemplate` _particulaspocionterminada "/Game/FXVarietyPack/Particles/P_ky_storm.P_ky_storm")
      (`ActorComponent.Activate` _particulaspocionterminada false)
      (`KismetSystemLibrary.PrintString` "Spawneando Pocion Mala")
      (`KismetSystemLibrary.Delay` 1.0)
      (bind _returnvalue (`|SpawnActorFromClass` "/Game/Blueprints/BP_Pociones/BP_Pociones_Child_Mala.BP_Pociones_Child_Mala_C" (`KismetMathLibrary.Conv_VectorToTransform` (`self.K2_GetActorLocation` (`self.PosicionSpawnPocion`))) "Undefined" "MultiplyWithRoot" null null))
      (bind _output_get (set `self.RefPocionMala` _returnvalue))
      (bind _staticmesh (`/Game/Blueprints/BP_Pociones/BP_Pociones.StaticMesh` _output_get))
      (`PrimitiveComponent.SetSimulatePhysics` _staticmesh true)
      (`PrimitiveComponent.AddImpulse` _staticmesh (500.0 500.0 500.0) "None" false)
      (`KismetSystemLibrary.Delay` 2.0)
      (`ActorComponent.Deactivate` (`self.ParticulasPocionTerminada`))
      (set `self.PocionMalaTerminada` true)
      (`GameplayStatics.PlaySound2D` "/Game/Audios/AudiosBolaCristal/CrearPocionMala.CrearPocionMala" 1.0 1.0 0.0 null null)
      (else
        (`KismetSystemLibrary.Delay` 1.0)
        (`self.ComprobarPocionMala`)))
    (elif (not (or (`self.PocionInvisibilidadTerminada`) (`self.PocionAmorTerminada`)))
      (goto _label))))

(event `self.Box.OnComponentBeginOverlap`
  (params (OverlappedComponent :type "PrimitiveComponent Object Reference") (OtherActor :type "Actor Object Reference") (OtherComp :type "PrimitiveComponent Object Reference") (OtherBodyIndex :type Integer) (bFromSweep :type Boolean) (SweepResult :type "HitResult Structure (by ref)"))
  (bind _efectodestruido (`self.EfectoDestruido`))
  ; Destruir Objeto Al Meterlo En Caldero
  (if (`KismetStringLibrary.EqualEqual_StrStr` (`KismetSystemLibrary.GetObjectName` OtherActor) (`KismetSystemLibrary.GetObjectName` (`|GetArrayItem` (`self.Viales`))))
    (`KismetArrayLibrary.Array_Clear` (`self.IngredientesEnCaldero`))
    (`NiagaraFunctionLibrary.SpawnSystemAtLocation` "/Game/KTP_Effect/Particles/Fly/Others/Trail_02_02.Trail_02_02" (`SceneComponent.RelativeLocation` _efectodestruido) (`SceneComponent.RelativeRotation` _efectodestruido))
    (`KismetSystemLibrary.Delay` 1.0)
    (`self.K2_DestroyActor` OtherActor)
    (for _array_element (`self.IngredientesEnCaldero`)
      (`KismetSystemLibrary.PrintString` (`KismetSystemLibrary.GetDisplayName` _array_element))
      (`KismetSystemLibrary.PrintString` "Array Ingredientes en caldero limpio"))
    (else
      (for _array_element_2 (`self.ArrayIngredientes`)
        (if (== OtherActor _array_element_2)
          (`ActorComponent.Activate` (`self.EfectoDestruido`) false)
          (`self.K2_DestroyActor` _array_element_2)
          (`KismetSystemLibrary.PrintString` "Ingrediente destruido")
          (set `self.NuevoIngredienteEnCaldero` true)
          (`/Engine/EditorBlueprintResources/StandardMacros.DoOnce` false
            (:`Completed`
              (set `self.ActivarContador` true)
              (`self.ComprobarTiempo`)
              (set `self.CalderoEnFuncionamiento` true))))))))

(event `ComprobarTiempo`
  ; Comprobar si el contador a acabo
  (if (<= (`/Game/Blueprints/BP_Contador/BP_Contador.TiempoRestante` (`self.Ref Contador`)) 0)
    (set `self.ElTiempoAAcabado?` true)
    (`KismetSystemLibrary.Delay` 10.0)
    (`self.Final`)
    (else
      (`KismetSystemLibrary.Delay` 0.2)
      (`self.ComprobarTiempo`))))

(event `Final`
  (if (`self.PocionAmorTerminada`)
    _
    (elif (`self.PocionInvisibilidadTerminada`)
      _)))

(fn `UserConstructionScript`)